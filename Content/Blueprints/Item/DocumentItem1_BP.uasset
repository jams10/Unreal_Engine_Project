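; Readable document pickup actor that shows its DocumentWidget on screen when the player interacts with it in range.
; CollisionVolume overlaps with ShooterCharacter_BP set a range flag and bind the interact event to player 0's character via AssignInteract.
; Interacting adds the widget to the viewport once and plays a paper sound.
; Leaving the volume clears the flag and removes the widget, but leaves the binding in place.
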(event OnComponentBeginOverlap(CollisionVolume)
  (params (OverlappedComponent :type Primitive%20Component%20Object%20Reference) (OtherActor :type Actor%20Object%20Reference) (OtherComp :type Primitive%20Component%20Object%20Reference) (OtherBodyIndex :type Integer) (bFromSweep :type Boolean) (SweepResult :type Hit%20Result%20Structure%20%28by%20ref%29))
  (Utilities|Casting|CastToShooterCharacter_BP OtherActor)
  (Variables|Default|SetPlayerIsInInteractiveRange true)
  (bind _asshooter_character_bp (Utilities|Casting|CastToShooterCharacter_BP (Game|GetPlayerCharacter 0)))
  (EventDispatchers|AssignInteract _asshooter_character_bp (delegate Custom|Interact_Event_0)))

(event OnComponentEndOverlap(CollisionVolume)
  (params (OverlappedComponent :type Primitive%20Component%20Object%20Reference) (OtherActor :type Actor%20Object%20Reference) (OtherComp :type Primitive%20Component%20Object%20Reference) (OtherBodyIndex :type Integer))
  (bind _documentwidget (Variables|Default|GetDocumentWidget))
  (Utilities|Casting|CastToShooterCharacter_BP OtherActor)
  (Variables|Default|SetPlayerIsInInteractiveRange false)
  (if (UserInterface|Viewport|IsinViewport _documentwidget)
    (Widget|RemovefromParent _documentwidget)))

(event Custom|Interact_Event_0
  (bind _documentwidget (Variables|Default|GetDocumentWidget))
  (if (Variables|Default|GetPlayerIsInInteractiveRange)
    (if (not (UserInterface|Viewport|IsinViewport _documentwidget))
      (UserInterface|Viewport|AddtoViewport _documentwidget 0)
      (Audio|PlaySound2D "/Game/Assets/Sounds/PaperSound.PaperSound" 1.0 1.0 0.0 0 0))))

(event EventBeginPlay)

(event Collision|EventActorBeginOverlap
  (params (OtherActor :type Actor%20Object%20Reference)))

(event EventTick
  (params (DeltaSeconds :type Float%20%28single-precision%29)))

(fn ConstructionScript)