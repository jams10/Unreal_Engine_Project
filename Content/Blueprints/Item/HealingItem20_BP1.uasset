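; HealingItem20_BP1 is a healing item pickup that the player can collect into the inventory.
; On BeginPlay it binds to the player character's PickupItem dispatcher.
; When that fires with collision enabled and IsInRange true, it adds itself to the controller's Inventory and refreshes the MainHUD inventory.
; It then hides itself and disables collision rather than being destroyed, and plays a pills pickup sound; no healing logic appears here.
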(event Custom|PickupItem_Event_0
  ;[1 1 1] 아이템 픽업
  (if (and (Collision|GetActorEnableCollision) (Variables|Default|GetbIsInRange))
    (bind _asshooter_player_controller_bp (Utilities|Casting|CastToShooterPlayerController_BP (Game|GetPlayerController 0)))
    (Utilities|Array|Add (Variables|/Game/Blueprints/ShooterPlayerController_BP.ShooterPlayerController_BP_C|GetInventory _asshooter_player_controller_bp) self)
    (bind _asshooter_player_controller_bp_2 (Utilities|Casting|CastToShooterPlayerController_BP (Game|GetPlayerController 0)))
    (bind _asmain_hud_bp (Utilities|Casting|CastToMainHUD_BP (Variables|/Script/The_Call.ShooterPlayerController|GetMainHUD _asshooter_player_controller_bp_2)))
    (Default|RefreshInventory (Variables|/Game/HUD/MainHUD_BP.MainHUD_BP_C|GetInventory _asmain_hud_bp))
    (Rendering|SetActorHiddenInGame true)
    (Collision|SetActorEnableCollision false)
    (Collision|SetCollisionEnabled (Variables|Default|GetCollisionVolume) "NoCollision")
    (Audio|PlaySoundatLocation "/Game/Assets/Sounds/PickupPills.PickupPills" (Transformation|GetActorLocation) "0, 0, 0" 1.0 1.0 0.0 0 0 0)))

(event EventBeginPlay
  (bind _asshooter_character_bp (Utilities|Casting|CastToShooterCharacter_BP (Game|GetPlayerCharacter 0)))
  (bind _output_get (Variables|Default|SetPlayer%20Reference _asshooter_character_bp))
  (EventDispatchers|AssignPickupItem _output_get (delegate Custom|PickupItem_Event_0)))

(event Collision|EventActorBeginOverlap
  (params (OtherActor :type Actor%20Object%20Reference)))

(event EventTick
  (params (DeltaSeconds :type Float%20%28single-precision%29)))

(fn ConstructionScript)