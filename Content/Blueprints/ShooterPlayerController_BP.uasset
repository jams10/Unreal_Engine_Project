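; Player controller for the shooter that manages the pause menu and relays inventory refreshes to the HUD.
; It creates the PauseHUD widget on BeginPlay, and P calls TogglePauseMenu, where a FlipFlop alternately shows or removes it while switching pause state, input mode and mouse cursor.
; RefreshInventory casts the stored MainHUD reference to MainHUD_BP and forwards the refresh to its Inventory widget.
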(event Custom|TogglePauseMenu
  (bind _returnvalue (Game|GetPlayerController 0))
  (bind _returnvalue_2 (Game|GetPlayerController 0))
  (Utilities|FlowControl|FlipFlop
    (:A
      (UserInterface|Viewport|AddtoViewport (Variables|Default|GetPauseUI) 0)
      (Input|SetInputModeGameandUI _returnvalue_2 0 "DoNotLock" true)
      (Variables|/Script/Engine.PlayerController|SetbShowMouseCursor _returnvalue_2 true)
      (Game|SetGamePaused true))
    (:B
      (Widget|RemovefromParent (Variables|Default|GetPauseUI))
      (Game|SetGamePaused false)
      (Input|SetInputModeGameOnly _returnvalue)
      (Variables|/Script/Engine.PlayerController|SetbShowMouseCursor _returnvalue false))))

(event EventBeginPlay
  (bind _returnvalue (UserInterface|CreateWidget "/Game/HUD/PauseHUD.PauseHUD_C"))
  (Variables|Default|SetPauseUI _returnvalue))

(event EventTick
  (params (DeltaSeconds :type Float%20%28single-precision%29)))

(event EventRefreshInventory
  (bind _asmain_hud_bp (Utilities|Casting|CastToMainHUD_BP (Variables|Default|GetMainHUD)))
  (Default|RefreshInventory (Variables|/Game/HUD/MainHUD_BP.MainHUD_BP_C|GetInventory _asmain_hud_bp)))

(event Input|KeyboardEvents|P
  (params (Key :type Key%20Structure :default "None"))
  (:Pressed
    (CallFunction|TogglePauseMenu)))

(fn ConstructionScript)