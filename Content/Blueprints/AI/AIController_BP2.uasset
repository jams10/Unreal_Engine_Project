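; AI controller for a slow zombie enemy that runs the BT_Zombie_Slow behavior tree on BeginPlay.
; Perception updates on the shooter player write CanSeePlayer, TargetActor and PatrolLocation to the Blackboard, including when sight is lost, so PatrolLocation holds the player's position at that moment.
; Tick polls the controlled enemy and stops the brain logic once it is dead.
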(event OnTargetPerceptionUpdated(AIPerception)
  (params (Actor :type Actor%20Object%20Reference) (Stimulus :type AI%20Stimulus%20Structure))
  (bind _asshooter_character_bp (Utilities|Casting|CastToShooterCharacter_BP Actor))
  (Utilities|IsValid _asshooter_character_bp
    (:Is%20Valid
      (Variables|Default|SetAs%20BP%20Shooter%20Character _asshooter_character_bp)
      ;[1 1 1] CanSeePlayer 키 Value 설정
      (AI|Components|Blackboard|SetValueasBool (Variables|Default|GetBlackboard) (Utilities|Name|MakeLiteralName "CanSeePlayer") (.bSuccessfullySensed (Utilities|Struct|BreakAIStimulus Stimulus)))
      ;[1 1 1] TargetActor 키 Value 설정
      (AI|Components|Blackboard|SetValueasObject (Variables|Default|GetBlackboard) (Utilities|Name|MakeLiteralName "TargetActor") (Variables|Default|GetAs%20BP%20Shooter%20Character))
      ;[1 1 1] PatrolLocation 키 Value 설정
      (AI|Components|Blackboard|SetValueasVector (Variables|Default|GetBlackboard) (Utilities|Name|MakeLiteralName "PatrolLocation") (Transformation|GetActorLocation (Variables|Default|GetAs%20BP%20Shooter%20Character))))))

(event EventBeginPlay
  (AI|RunBehaviorTree "/Game/Blueprints/AI/BehaviorTree/BT_Zombie_Slow.BT_Zombie_Slow"))

(event EventTick
  (params (DeltaSeconds :type Float%20%28single-precision%29))
  (bind _asenemy_character (Utilities|Casting|CastToEnemyCharacter (Pawn|GetControlledPawn)))
  (if (Class|EnemyCharacter|IsDead _asenemy_character)
    (AI|Logic|StopLogic (Variables|Default|GetBrainComponent) "Dead")))

(fn ConstructionScript)