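; Player character Blueprint for a shooter, handling the flashlight, item pickup, inventory screen and starting pistol.
; Tick aims the flashlight along the controller's rotation and, once, spawns and equips the pistol there rather than in BeginPlay, which failed in packaged builds.
; E calls interact while the controller's inventory has room, and F toggles the light.
; The inventory input flips the HUD panel with animation, sound and cursor/input-mode switching.
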(event Custom|ToggleInventory
  (bind _mainhud_bp_reference (Variables|Default|GetMainHUD_BP%20Reference))
  (bind _mainhud_bp_reference_2 (Variables|Default|GetMainHUD_BP%20Reference))
  ;[1 1 1] 인벤토리 메뉴 토글
  (Utilities|FlowControl|FlipFlop
    (:A
      (Audio|PlaySound2D "/Engine/VREditor/Sounds/UI/Dockable_Window_Open.Dockable_Window_Open" 1.0 1.0 0.0 0 0)
      (Widget|SetVisibility (Variables|/Game/HUD/MainHUD_BP.MainHUD_BP_C|GetInventory _mainhud_bp_reference_2) "Visible")
      (UserInterface|Animation|PlayAnimation _mainhud_bp_reference_2 (Variables|/Game/HUD/MainHUD_BP.MainHUD_BP_C|GetInventoryAnim _mainhud_bp_reference_2) 0.0 1 "Forward" 1.0 false)
      (CallFunction|EnableMouseCursorandInputUIandGameOnly)
      (Variables|Default|SetbInventoryIsOpen true))
    (:B
      (Audio|PlaySound2D "/Engine/VREditor/Sounds/UI/Dockable_Window_Close.Dockable_Window_Close" 1.0 1.0 0.0 0 0)
      (UserInterface|Animation|PlayAnimation _mainhud_bp_reference (Variables|/Game/HUD/MainHUD_BP.MainHUD_BP_C|GetInventoryAnim _mainhud_bp_reference) 0.0 1 "Reverse" 1.0 false)
      (CallFunction|DisableMouseCursorandInputGameOnly)
      (Widget|SetVisibility (Variables|/Game/HUD/MainHUD_BP.MainHUD_BP_C|GetInventory _mainhud_bp_reference) "Hidden")
      (Variables|Default|SetbInventoryIsOpen false))))

(event EventBeginPlay)

(event Collision|EventActorBeginOverlap
  (params (OtherActor :type Actor%20Object%20Reference)))

(event EventTick
  (params (DeltaSeconds :type Float%20%28single-precision%29))
  ;[1 1 1] 플레이어가 바라보는 방향으로 라이트 회전을 설정함.
  (Transformation|SetWorldRotation (Variables|Default|GetFlashLight) (Transformation|GetActorRotation (Game|GetPlayerController 0)) false false)
  ;[1 1 1] 시작할 때 총 하나를 들고 시작. 에디터 상에서는 Begin Play에 연결해도 동작에 문제가 없는데, ㅅ실제 빌드를 하여 게임을 실행했을 때 제대로 동작되지 않았음. 총 블루프린트나 위젯 블루프린트의 생성 시점들이 서로 엇갈려서 제대로 동작되지 않는 것 같음.
  (Utilities|FlowControl|DoOnce false
    (:Completed
      (bind _returnvalue (Game|SpawnActorfromClass "/Game/Blueprints/Item/PistolItem_BP.PistolItem_BP_C" (Transformation|GetActorTransform) "Undefined" 0 0))
      (bind _output_get (Variables|Default|SetPistolForStart _returnvalue))
      (Collision|SetActorEnableCollision _output_get false)
      (Collision|SetCollisionEnabled (Variables|/Script/The_Call.PickupItem|GetCollisionVolume _output_get) "NoCollision")
      (bind _asshooter_player_controller_bp (Utilities|Casting|CastToShooterPlayerController_BP (Game|GetPlayerController 0)))
      (Utilities|Array|Add (Variables|/Script/The_Call.ShooterPlayerController|GetInventory _asshooter_player_controller_bp) (Variables|Default|GetPistolForStart))
      (bind _asmain_hud_bp (Utilities|Casting|CastToMainHUD_BP (Variables|/Script/The_Call.ShooterPlayerController|GetMainHUD _asshooter_player_controller_bp)))
      (Variables|Default|SetMainHUD_BP%20Reference _asmain_hud_bp)
      (Default|RefreshInventory (Variables|/Game/HUD/MainHUD_BP.MainHUD_BP_C|GetInventory _asmain_hud_bp))
      (bind _asshooter_character_bp (Utilities|Casting|CastToShooterCharacter_BP (Game|GetPlayerCharacter 0)))
      (Class|ShooterCharacter|SetCurrentHoldingGun _asshooter_character_bp (Variables|Default|GetPistolForStart)))))

(event Input|ActionEvents|InputActionToggleInventory
  (params (Key :type Key%20Structure :default "None"))
  ;[1 1 1] 인벤토리 메뉴 토글
  (:Pressed
    (CallFunction|ToggleInventory)))

(event Input|KeyboardEvents|E
  (params (Key :type Key%20Structure :default "None"))
  ;[1 1 1] 아이템 픽업
  (:Pressed
    (bind _asshooter_player_controller_bp (Utilities|Casting|CastToShooterPlayerController_BP (Game|GetPlayerController 0)))
    (if (< (Utilities|Array|Length (Variables|/Game/Blueprints/ShooterPlayerController_BP.ShooterPlayerController_BP_C|GetInventory _asshooter_player_controller_bp)) 15)
      (Default|CallInteract))))

(event Input|KeyboardEvents|F
  (params (Key :type Key%20Structure :default "None"))
  (:Pressed
    (Utilities|FlowControl|FlipFlop
      (:A
        (Rendering|SetVisibility (Variables|Default|GetFlashLight) true false))
      (:B
        (Rendering|SetVisibility (Variables|Default|GetFlashLight) false false)))
    (Audio|PlaySoundatLocation "/Game/Assets/Sounds/Gun/ClickSound.ClickSound" (Transformation|GetActorLocation) "0, 0, 0" 1.0 1.0 0.0 0 0 0)))

(fn ConstructionScript)

(fn EnableMouseCursorandInputUIandGameOnly
  (bind _returnvalue (Game|GetPlayerController 0))
  (Input|SetInputModeGameandUI _returnvalue (Variables|Default|GetMainHUD_BP%20Reference) "DoNotLock" true)
  (Variables|/Script/Engine.PlayerController|SetbShowMouseCursor _returnvalue true))

(fn DisableMouseCursorandInputGameOnly
  (bind _returnvalue (Game|GetPlayerController 0))
  (Input|SetInputModeGameOnly _returnvalue)
  (Variables|/Script/Engine.PlayerController|SetbShowMouseCursor _returnvalue false))