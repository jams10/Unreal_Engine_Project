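; PhysicsDoor_BP is a door that swings itself back to its starting rotation when no Character is nearby.
; It records the door's world rotation at BeginPlay.
; Overlap events on a closing-range volume set a presence flag, and while that is clear, Tick eases the door back with RInterpTo.
; The flag is a single boolean, so any Character leaving clears it even if another remains inside.
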(event OnComponentBeginOverlap(CollisionVolumeForClosingDoor)
  (params (OverlappedComponent :type Primitive%20Component%20Object%20Reference) (OtherActor :type Actor%20Object%20Reference) (OtherComp :type Primitive%20Component%20Object%20Reference) (OtherBodyIndex :type Integer) (bFromSweep :type Boolean) (SweepResult :type Hit%20Result%20Structure%20%28by%20ref%29))
  (Utilities|Casting|CastToCharacter OtherActor)
  (Variables|Default|SetSomeoneIsInClosingDoorRange true))

(event OnComponentEndOverlap(CollisionVolumeForClosingDoor)
  (params (OverlappedComponent :type Primitive%20Component%20Object%20Reference) (OtherActor :type Actor%20Object%20Reference) (OtherComp :type Primitive%20Component%20Object%20Reference) (OtherBodyIndex :type Integer))
  (Utilities|Casting|CastToCharacter OtherActor)
  (Variables|Default|SetSomeoneIsInClosingDoorRange false))

(event EventBeginPlay
  (Variables|Default|SetOriginRotation (Transformation|GetWorldRotation (Variables|Default|GetDoor))))

(event Collision|EventActorBeginOverlap
  (params (OtherActor :type Actor%20Object%20Reference)))

(event EventTick
  (params (DeltaSeconds :type Float%20%28single-precision%29))
  (bind _door (Variables|Default|GetDoor))
  (if (not (Variables|Default|GetSomeoneIsInClosingDoorRange))
    (Transformation|SetWorldRotation _door (Math|Interpolation|RInterpTo (Transformation|GetWorldRotation _door) (Variables|Default|GetOriginRotation) DeltaSeconds 1.0) false false)))

(fn ConstructionScript)