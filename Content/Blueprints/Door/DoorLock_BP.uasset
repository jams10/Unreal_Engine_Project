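; Door lock actor that opens a linked DoorLockPhysicsDoor_BP when its password is matched.
; Entering its box shows an interact prompt, screen-projected each Tick, and assigns the character's interact event to open the DoorLock widget with a cursor.
; The widget receives a self reference, and Tick polls the match and incorrect flags to play a sound, close the UI and restore game input.
; A match also sets the door's HasOpend and destroys the interaction box.
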(event OnComponentBeginOverlap(BoxCollisionForInteract)
  (params (OverlappedComponent :type Primitive%20Component%20Object%20Reference) (OtherActor :type Actor%20Object%20Reference) (OtherComp :type Primitive%20Component%20Object%20Reference) (OtherBodyIndex :type Integer) (bFromSweep :type Boolean) (SweepResult :type Hit%20Result%20Structure%20%28by%20ref%29))
  (bind _asshooter_character_bp (Utilities|Casting|CastToShooterCharacter_BP OtherActor))
  (Variables|Default|SetPlayerIsInInteractRange true)
  (UserInterface|Viewport|AddtoViewport (Variables|Default|GetInteractUI) 0)
  (EventDispatchers|AssignInteract _asshooter_character_bp (delegate Custom|Interact_Event_0)))

(event OnComponentEndOverlap(BoxCollisionForInteract)
  (params (OverlappedComponent :type Primitive%20Component%20Object%20Reference) (OtherActor :type Actor%20Object%20Reference) (OtherComp :type Primitive%20Component%20Object%20Reference) (OtherBodyIndex :type Integer))
  (bind _returnvalue (Game|GetPlayerController 0))
  (Utilities|Casting|CastToShooterCharacter_BP OtherActor)
  (Variables|Default|SetPlayerIsInInteractRange false)
  (Widget|RemovefromParent (Variables|Default|GetDoorLockUI))
  (Input|SetInputModeGameOnly _returnvalue)
  (Variables|/Script/Engine.PlayerController|SetbShowMouseCursor _returnvalue false)
  (if (UserInterface|Viewport|IsinViewport (Variables|Default|GetInteractUI))
    (Widget|RemovefromParent (Variables|Default|GetInteractUI))))

(event Custom|Interact_Event_0
  (bind _returnvalue (Game|GetPlayerController 0))
  (if (Variables|Default|GetPlayerIsInInteractRange)
    (if (not (UserInterface|Viewport|IsinViewport (Variables|Default|GetDoorLockUI)))
      (Input|SetInputModeGameandUI _returnvalue 0 "DoNotLock" true)
      (Variables|/Script/Engine.PlayerController|SetbShowMouseCursor _returnvalue true)
      (Audio|PlaySound2D "/Engine/VREditor/Sounds/UI/Click_on_Button.Click_on_Button" 1.0 1.0 0.0 0 0)
      (UserInterface|Viewport|AddtoViewport (Variables|Default|GetDoorLockUI) 0)
      (Widget|RemovefromParent (Variables|Default|GetInteractUI)))))

(event EventBeginPlay
  (bind _returnvalue (UserInterface|CreateWidget "/Game/HUD/DoorLock.DoorLock_C" 0 self))
  (Variables|Default|SetDoorLockUI _returnvalue)
  (bind _returnvalue_2 (UserInterface|CreateWidget "/Game/HUD/InteractiveTextOverlay.InteractiveTextOverlay_C"))
  (Variables|Default|SetInteractUI _returnvalue_2))

(event Collision|EventActorBeginOverlap
  (params (OtherActor :type Actor%20Object%20Reference)))

(event EventTick
  (params (DeltaSeconds :type Float%20%28single-precision%29))
  (bind _returnvalue (Game|GetPlayerController 0))
  (bind _returnvalue_2 (Transformation|GetActorLocation))
  (bind _returnvalue_3 (Game|GetPlayerController 0))
  (bind _returnvalue_4 (+ _returnvalue_2 "0, 0,20.000000"))
  (bind (_screenlocation _returnvalue_5) (Class|PlayerController|ProjectWorldLocationtoScreen _returnvalue_3 _returnvalue_4 false))
  (Utilities|FlowControl|Sequence
    (:then_0
      (if _returnvalue_5
        (Class|UserWidget|SetPositioninViewport (Variables|Default|GetInteractUI) _screenlocation true)))
    (:then_1
      ;[1 1 1] 패스 워드 일치의 경우(레퍼런스로 받아온 문의 HasOpend 변수를 true로 변경하여 문이 열리도록 함.)
      (if (Variables|Default|GetPasswordHasMatched)
        (Audio|PlaySound2D "/Engine/EditorSounds/Notifications/CompileSuccess.CompileSuccess" 0.4 1.0 0.0 0 0)
        (Variables|Default|SetPasswordHasMatched false)
        (if (UserInterface|Viewport|IsinViewport (Variables|Default|GetDoorLockUI))
          (Widget|RemovefromParent (Variables|Default|GetDoorLockUI))
          (bind _asdoor_lock_physics_door_bp (Utilities|Casting|CastToDoorLockPhysicsDoor_BP (Variables|Default|GetDoor)))
          (Variables|/Game/Blueprints/Door/DoorLockPhysicsDoor_BP.DoorLockPhysicsDoor_BP_C|SetHasOpend _asdoor_lock_physics_door_bp true)
          (Components|DestroyComponent (Variables|Default|GetBoxCollisionForInteract))
          ;[1 1 1] 인풋을 다시 게임 인풋으로 되돌리고 마우스 커서 숨김.
          (Input|SetInputModeGameOnly _returnvalue :!label _label)
          (Variables|/Script/Engine.PlayerController|SetbShowMouseCursor _returnvalue false))))
    (:then_2
      ;[1 1 1] 패스워드 불일치의 경우
      (if (Variables|Default|GetPasswordIncorrect)
        (Audio|PlaySound2D "/Engine/EditorSounds/Notifications/CompileFailed.CompileFailed" 0.4 1.0 0.0 0 0)
        (Variables|Default|SetPasswordIncorrect false)
        (if (UserInterface|Viewport|IsinViewport (Variables|Default|GetDoorLockUI))
          (Widget|RemovefromParent (Variables|Default|GetDoorLockUI))
          (goto _label))))))

(fn ConstructionScript)