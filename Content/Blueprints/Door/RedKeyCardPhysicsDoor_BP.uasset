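; Physics door that stays locked until the player uses a red key card on it.
; Entering the key card box shows a prompt and binds Interact to toggle the inventory.
; Tick polls inventory for used keys, enabling door physics for red or playing a locked sound otherwise.
; Tick also projects the prompt to screen and, when that succeeds, eases the door back to its original rotation if no Character occupies the closing volume.
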(event OnComponentBeginOverlap(CollisionVolumeForClosingDoor)
  (params (OverlappedComponent :type Primitive%20Component%20Object%20Reference) (OtherActor :type Actor%20Object%20Reference) (OtherComp :type Primitive%20Component%20Object%20Reference) (OtherBodyIndex :type Integer) (bFromSweep :type Boolean) (SweepResult :type Hit%20Result%20Structure%20%28by%20ref%29))
  ;[1 1 1] 플레이어가 주위에 없을 경우 자동으로 문이 닫히도록 Overlap 이벤트 구성
  (Utilities|Casting|CastToCharacter OtherActor)
  (Variables|Default|SetSomeoneIsInClosingDoorRange true))

(event OnComponentEndOverlap(CollisionVolumeForClosingDoor)
  (params (OverlappedComponent :type Primitive%20Component%20Object%20Reference) (OtherActor :type Actor%20Object%20Reference) (OtherComp :type Primitive%20Component%20Object%20Reference) (OtherBodyIndex :type Integer))
  ;[1 1 1] 플레이어가 주위에 없을 경우 자동으로 문이 닫히도록 Overlap 이벤트 구성
  (Utilities|Casting|CastToCharacter OtherActor)
  (Variables|Default|SetSomeoneIsInClosingDoorRange false))

(event OnComponentBeginOverlap(BoxCollisionForKeyCardCheck)
  (params (OverlappedComponent :type Primitive%20Component%20Object%20Reference) (OtherActor :type Actor%20Object%20Reference) (OtherComp :type Primitive%20Component%20Object%20Reference) (OtherBodyIndex :type Integer) (bFromSweep :type Boolean) (SweepResult :type Hit%20Result%20Structure%20%28by%20ref%29))
  (Utilities|Casting|CastToShooterCharacter OtherActor)
  (UserInterface|Viewport|AddtoViewport (Variables|Default|GetInteractionOverlay) 0)
  (Variables|Default|SetPlayerIsInInteractiveRange true)
  (bind _asshooter_character_bp (Utilities|Casting|CastToShooterCharacter_BP (Game|GetPlayerCharacter 0)))
  (EventDispatchers|AssignInteract _asshooter_character_bp (delegate Custom|TryOpenDoor)))

(event OnComponentEndOverlap(BoxCollisionForKeyCardCheck)
  (params (OverlappedComponent :type Primitive%20Component%20Object%20Reference) (OtherActor :type Actor%20Object%20Reference) (OtherComp :type Primitive%20Component%20Object%20Reference) (OtherBodyIndex :type Integer))
  (Utilities|Casting|CastToShooterCharacter OtherActor)
  (Widget|RemovefromParent (Variables|Default|GetInteractionOverlay))
  (Variables|Default|SetPlayerIsInInteractiveRange false))

(event Custom|TryOpenDoor
  (if (Variables|Default|GetPlayerIsInInteractiveRange)
    (bind _asshooter_character_bp (Utilities|Casting|CastToShooterCharacter_BP (Game|GetPlayerCharacter 0)))
    (Default|ToggleInventory _asshooter_character_bp)))

(event EventBeginPlay
  (bind _door (Variables|Default|GetDoor))
  (Variables|Default|SetOriginRotation (Transformation|GetWorldRotation _door))
  (Physics|SetSimulatePhysics _door false)
  (bind _returnvalue (UserInterface|CreateWidget "/Game/HUD/InteractiveTextOverlay.InteractiveTextOverlay_C"))
  (Variables|Default|SetInteractionOverlay _returnvalue))

(event Collision|EventActorBeginOverlap
  (params (OtherActor :type Actor%20Object%20Reference)))

(event EventTick
  (params (DeltaSeconds :type Float%20%28single-precision%29))
  (bind _returnvalue (Transformation|GetActorLocation))
  (bind _returnvalue_2 (Game|GetPlayerController 0))
  (bind _interactionoverlay (Variables|Default|GetInteractionOverlay))
  (bind _door (Variables|Default|GetDoor))
  (bind _returnvalue_3 (+ _returnvalue "0, 0,100.000000"))
  (bind (_screenlocation _returnvalue_4) (Class|PlayerController|ProjectWorldLocationtoScreen _returnvalue_2 _returnvalue_3 false))
  (if (and (Variables|Default|GetPlayerIsInInteractiveRange) (not (Class|SceneComponent|IsAnySimulatingPhysics (Variables|Default|GetDoor))))
    ;[1 1 1] 인벤토리에 키가 있고 해당 사용 했는지와 키의 타입을 체크
    (bind _asshooter_player_controller (Utilities|Casting|CastToShooterPlayerController (Game|GetPlayerController 0)))
    (for _array_element (Variables|/Script/The_Call.ShooterPlayerController|GetInventory _asshooter_player_controller)
      (bind _askey_item (Utilities|Casting|CastToKeyItem _array_element))
      (if (and (Variables|/Script/The_Call.KeyItem|GetbPlayerHasUsed _askey_item) (Utilities|Enum|Equal(Enum) (Class|KeyItem|GetKeyType _askey_item) "KT_RED"))
        (Variables|/Script/The_Call.KeyItem|SetbPlayerHasUsed _askey_item false)
        (Physics|SetSimulatePhysics (Variables|Default|GetDoor) true)
        (if (UserInterface|Viewport|IsinViewport _interactionoverlay)
          (Widget|RemovefromParent _interactionoverlay)
          (Components|DestroyComponent (Variables|Default|GetBoxCollisionForKeyCardCheck))
          (Audio|PlaySoundatLocation "/Game/Assets/Sounds/DoorUnlock.DoorUnlock" (Transformation|GetActorLocation) "0, 0, 0" 1.0 1.0 0.0 0 0 0))
        (elif (Variables|/Script/The_Call.KeyItem|GetbPlayerHasUsed _askey_item)
          (Audio|PlaySoundatLocation "/Game/Assets/Sounds/DoorLock.DoorLock" (Transformation|GetActorLocation) "0, 0, 0" 1.0 1.0 0.0 0 0 0)
          (Variables|/Script/The_Call.KeyItem|SetbPlayerHasUsed _askey_item false))))
    (else
      ;[1 1 1] 오버레이 위젯이 플레이어를 바라보게 함.
      (if _returnvalue_4
        (Class|UserWidget|SetPositioninViewport (Variables|Default|GetInteractionOverlay) _screenlocation true)
        ;[1 1 1] 범위에 플레이어 없으면 문 닫기
        (if (not (Variables|Default|GetSomeoneIsInClosingDoorRange))
          (Transformation|SetWorldRotation _door (Math|Interpolation|RInterpTo (Transformation|GetWorldRotation _door) (Variables|Default|GetOriginRotation) DeltaSeconds 1.0) false false))))))

(fn ConstructionScript)