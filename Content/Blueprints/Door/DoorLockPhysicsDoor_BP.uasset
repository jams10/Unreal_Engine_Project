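; Password-locked physics door Blueprint that stays non-simulated until unlocked and drifts back to its original rotation.
; BeginPlay stores the door's rotation; once HasOpend is true (password matched, per the comment), Tick plays an opening sound and enables physics a single time.
; A collision volume tracks Characters, and while none is flagged inside, Tick interpolates the door back to that stored rotation.
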(event OnComponentBeginOverlap(CollisionVolumeForClosingDoor)
  (params (OverlappedComponent :type Primitive%20Component%20Object%20Reference) (OtherActor :type Actor%20Object%20Reference) (OtherComp :type Primitive%20Component%20Object%20Reference) (OtherBodyIndex :type Integer) (bFromSweep :type Boolean) (SweepResult :type Hit%20Result%20Structure%20%28by%20ref%29))
  (Utilities|Casting|CastToCharacter OtherActor)
  (Variables|Default|SetSomeoneIsInClosingDoorRange true))

(event OnComponentEndOverlap(CollisionVolumeForClosingDoor)
  (params (OverlappedComponent :type Primitive%20Component%20Object%20Reference) (OtherActor :type Actor%20Object%20Reference) (OtherComp :type Primitive%20Component%20Object%20Reference) (OtherBodyIndex :type Integer))
  (Utilities|Casting|CastToCharacter OtherActor)
  (Variables|Default|SetSomeoneIsInClosingDoorRange false))

(event EventBeginPlay
  (Variables|Default|SetOriginRotation (Transformation|GetWorldRotation (Variables|Default|GetDoor)))
  (Physics|SetSimulatePhysics (Variables|Default|GetDoor) false))

(event Collision|EventActorBeginOverlap
  (params (OtherActor :type Actor%20Object%20Reference)))

(event EventTick
  (params (DeltaSeconds :type Float%20%28single-precision%29))
  (bind _door (Variables|Default|GetDoor))
  (Utilities|FlowControl|Sequence
    (:then_0
      ;[1 1 1] HasOpened = true 이면 패스워드가 일치했다는 것임. 따라서 문이 열리는 사운드 재생 후 피직스 시뮬레이션 키기
      (if (Variables|Default|GetHasOpend)
        (Utilities|FlowControl|DoOnce false
          (:Completed
            (Audio|PlaySoundatLocation "/Engine/VREditor/Sounds/UI/Dockable_Window_Open.Dockable_Window_Open" (Transformation|GetActorLocation) "0, 0, 0" 1.0 1.0 0.0 0 0 0)
            (Physics|SetSimulatePhysics (Variables|Default|GetDoor) true)))))
    (:then_1
      (if (not (Variables|Default|GetSomeoneIsInClosingDoorRange))
        (Transformation|SetWorldRotation _door (Math|Interpolation|RInterpTo (Transformation|GetWorldRotation _door) (Variables|Default|GetOriginRotation) DeltaSeconds 1.0) false false)))))

(fn ConstructionScript)